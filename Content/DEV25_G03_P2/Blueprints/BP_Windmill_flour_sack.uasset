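; BP_Windmill_flour_sack is a windmill delivery trigger that turns a full cart of barrels into flour sack progress.
; On overlap, it checks the third-cargo flag in the Game_Rules game instance, printing a shortage message if unset.
; If set and the overlapping actor is BP_Cart, it respawns the cart and sets the next unset flag of three sequential flour sack flags.
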(event Collision|EventActorBeginOverlap
  (params (OtherActor :type Actor%20Object%20Reference))
  (bind _asgame_rules (Utilities|Casting|CastToGame_Rules (Game|GetGameInstance)))
  (if (Variables|/Game/DEV25_G03_P2/Blueprints/Game_Rules.Game_Rules_C|GetCart_cargo_3_set _asgame_rules)
    (bind _asbp_cart (Utilities|Casting|CastToBP_Cart OtherActor))
    (Default|CartRespawn _asbp_cart)
    (bind _asgame_rules_2 (Utilities|Casting|CastToGame_Rules (Game|GetGameInstance)))
    (if (Variables|/Game/DEV25_G03_P2/Blueprints/Game_Rules.Game_Rules_C|GetFlour_sack_1_set _asgame_rules_2)
      (if (Variables|/Game/DEV25_G03_P2/Blueprints/Game_Rules.Game_Rules_C|GetFlour_sack_2_set _asgame_rules_2)
        (if (not (Variables|/Game/DEV25_G03_P2/Blueprints/Game_Rules.Game_Rules_C|GetFlour_sack_3_set _asgame_rules_2))
          (Variables|/Game/DEV25_G03_P2/Blueprints/Game_Rules.Game_Rules_C|SetFlour_sack_3_set _asgame_rules_2 true))
        (else
          (Variables|/Game/DEV25_G03_P2/Blueprints/Game_Rules.Game_Rules_C|SetFlour_sack_2_set _asgame_rules_2 true)))
      (else
        (Variables|/Game/DEV25_G03_P2/Blueprints/Game_Rules.Game_Rules_C|SetFlour_sack_1_set _asgame_rules_2 true)))
    (else
      (Development|PrintText "Not enough barrels, 3 needed"))))

(fn ConstructionScript)