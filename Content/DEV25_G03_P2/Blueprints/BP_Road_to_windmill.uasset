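; BP_Road_to_windmill is a road actor that tracks whether a BP_Cart stays on the road and respawns it when it leaves.
; Begin and end overlaps increment and decrement the cart's StayInRoadCounter, so overlapping several counted actors keeps it above zero.
; At zero or below, either event prints a warning, waits three seconds and calls CartRespawn, without rechecking the counter after the delay.
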(event Collision|EventActorBeginOverlap
  (params (OtherActor :type Actor%20Object%20Reference))
  ;[0.15 0.15 0.15 0.5] Road logic
  (bind _asbp_cart (Utilities|Casting|CastToBP_Cart OtherActor))
  (bind _output_get (Variables|/Game/DEV25_G03_P2/Blueprints/BP_Cart.BP_Cart_C|SetStay_in_road_counter _asbp_cart (+ (Variables|/Game/DEV25_G03_P2/Blueprints/BP_Cart.BP_Cart_C|GetStay_in_road_counter _asbp_cart) 1)))
  (if (<= _output_get 0)
    (Development|PrintString "Out of the road, self destruction in 3 seconds")
    (Utilities|FlowControl|Delay 3.0)
    (Default|CartRespawn _asbp_cart)))

(event Collision|EventActorEndOverlap
  (params (OtherActor :type Actor%20Object%20Reference))
  ;[0.15 0.15 0.15 0.5] Road logic
  (bind _asbp_cart (Utilities|Casting|CastToBP_Cart OtherActor))
  (bind _output_get (Variables|/Game/DEV25_G03_P2/Blueprints/BP_Cart.BP_Cart_C|SetStay_in_road_counter _asbp_cart (- (Variables|/Game/DEV25_G03_P2/Blueprints/BP_Cart.BP_Cart_C|GetStay_in_road_counter _asbp_cart) 1)))
  (if (<= _output_get 0)
    (Development|PrintString "Out of the road, self destruction in 3 seconds")
    (Utilities|FlowControl|Delay 3.0)
    (Default|CartRespawn _asbp_cart)))

(fn ConstructionScript)