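; BP_CartWheel is a flashing cart wheel that the player moves and rotates until the cart is fixed.
; Overlapping ClickArea, once Game_Rules has BaldosaSet, enables input and blends the camera to the wheel; leaving reverts both.
; Keys nudge its location and rotation in fixed steps, with sweep only on W/S moves.
; The flash timeline also polls CartFixed, then hides the wheel and disables its collision.
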(event OnComponentEndOverlap(clickArea)
  (params (OverlappedComponent :type Primitive%20Component%20Object%20Reference) (OtherActor :type Actor%20Object%20Reference) (OtherComp :type Primitive%20Component%20Object%20Reference) (OtherBodyIndex :type Integer))
  ;[0.15 0.15 0.15 0.5] Camera switch and inputs
  (Input|DisableInput 0)
  (Game|Player|SetViewTargetwithBlend (Game|GetPlayerController 0) (Game|GetPlayerCharacter 0) 0.0 "VTBlend_Linear" 0.0 false))

(event OnComponentBeginOverlap(clickArea)
  (params (OverlappedComponent :type Primitive%20Component%20Object%20Reference) (OtherActor :type Actor%20Object%20Reference) (OtherComp :type Primitive%20Component%20Object%20Reference) (OtherBodyIndex :type Integer) (bFromSweep :type Boolean) (SweepResult :type Hit%20Result%20Structure%20%28by%20ref%29))
  ;[0.15 0.15 0.15 0.5] Camera switch and inputs
  (Utilities|Casting|CastToBP_ABCharacter OtherActor)
  (bind _asgame_rules (Utilities|Casting|CastToGame_Rules (Game|GetGameInstance)))
  (if (Variables|/Game/DEV25_G03_P2/Blueprints/Game_Rules.Game_Rules_C|GetBaldosa_Set _asgame_rules)
    (Input|EnableInput (Game|GetPlayerController 0))
    (if (Actor|ActorHasTag OtherActor "ABPlayer")
      (Game|Player|SetViewTargetwithBlend (Game|GetPlayerController 0) self 0.0 "VTBlend_Linear" 0.0 false))))

(event Custom|wheelInstalled
  (Collision|SetActorEnableCollision false)
  (Rendering|SetActorHiddenInGame true))

(event EventBeginPlay
  ;[0.15 0.15 0.15 0.5] Let the wheel flash and read its coord
  (Variables|Default|SetCurrentLocation (Transformation|GetActorLocation))
  (bind _newtrack_2 (Timeline|wheelline Play)
    (:Update
      (Rendering|Components|Light|SetIntensity (Variables|Default|GetwheelFlash) (Math|Float|Lerp 1e+04 0.0 _newtrack_2))
      (bind _asgame_rules (Utilities|Casting|CastToGame_Rules (Game|GetGameInstance)))
      (if (Variables|/Game/DEV25_G03_P2/Blueprints/Game_Rules.Game_Rules_C|GetCart_fixed _asgame_rules)
        (CallFunction|WheelInstalled)))))

(event Input|KeyboardEvents|W
  (params (Key :type Key%20Structure :default "None"))
  ;[0.15 0.15 0.15 0.5] Input mapping for wheel
  (:Pressed
    (bind _output_get (Variables|Default|SetCurrentLocation (+ (Variables|Default|GetCurrentLocation) (Math|Vector|RotateVectorAroundAxis (* (Transformation|GetActorForwardVector) 1e+01) 9e+01 "0.000000,0.000000,1.000000"))))
    (Transformation|SetActorLocation _output_get true false)))

(event Input|KeyboardEvents|S
  (params (Key :type Key%20Structure :default "None"))
  ;[0.15 0.15 0.15 0.5] Input mapping for wheel
  (:Pressed
    (bind _output_get (Variables|Default|SetCurrentLocation (+ (Variables|Default|GetCurrentLocation) (Math|Vector|RotateVectorAroundAxis (* (Transformation|GetActorForwardVector) -1e+01) 9e+01 "0.000000,0.000000,1.000000"))))
    (Transformation|SetActorLocation _output_get true false)))

(event Input|KeyboardEvents|A
  (params (Key :type Key%20Structure :default "None"))
  ;[0.15 0.15 0.15 0.5] Input mapping for wheel
  (:Pressed
    (Transformation|AddActorLocalRotation "0.000000,-5.000000,0.000000" false false)))

(event Input|KeyboardEvents|D
  (params (Key :type Key%20Structure :default "None"))
  ;[0.15 0.15 0.15 0.5] Input mapping for wheel
  (:Pressed
    (Transformation|AddActorLocalRotation "0.000000,5.000000,0.000000" false false)))

(event Input|KeyboardEvents|Q
  (params (Key :type Key%20Structure :default "None"))
  ;[0.15 0.15 0.15 0.5] Input mapping for wheel
  (:Pressed
    (bind _output_get (Variables|Default|SetCurrentLocation (+ (Variables|Default|GetCurrentLocation) "0.000000,0.000000,10.000000")))
    (Transformation|SetActorLocation _output_get false false)))

(event Input|KeyboardEvents|E
  (params (Key :type Key%20Structure :default "None"))
  ;[0.15 0.15 0.15 0.5] Input mapping for wheel
  (:Pressed
    (bind _output_get (Variables|Default|SetCurrentLocation (+ (Variables|Default|GetCurrentLocation) "0.000000,0.000000,-10.000000")))
    (Transformation|SetActorLocation _output_get false false)))

(fn ConstructionScript)